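; BP_KeyCard is a pickup actor that gives the player a keycard.
; Each tick a sphere trace around the card looks for the player pawn, enabling pickup and toggling a guarded prompt widget.
; The pickup input attaches the card to a socket on the character mesh, disables collision, shows a confirmation widget and flags PlayerBase as holding the keycard.
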(event Custom|Add%20Pickup%20Keycard%20Widget%20to%20Viewport
  (if (not (Variables|Default|GetPickup%20Keycard%20Present))
    (bind _returnvalue (UserInterface|CreateWidget "/Game/MainLevelUI/PickupKeycardWidget.PickupKeycardWidget_C"))
    (UserInterface|Viewport|AddtoViewport _returnvalue 0)
    (Variables|Default|SetPickup%20Keycard%20Present true)))

(event Custom|Remove%20Pickup%20Keycard%20Widget%20from%20Viewport
  (if (Variables|Default|GetPickup%20Keycard%20Present)
    (if (Utilities|IsValid (stale Custom|Add%20Pickup%20Keycard%20Widget%20to%20Viewport _returnvalue))
      (Widget|RemovefromParent (stale Custom|Add%20Pickup%20Keycard%20Widget%20to%20Viewport _returnvalue))
      (Variables|Default|SetPickup%20Keycard%20Present false))))

(event EventBeginPlay)

(event Collision|EventActorBeginOverlap
  (params (OtherActor :type Actor%20Object%20Reference)))

(event EventTick
  (params (DeltaSeconds :type Float%20%28single-precision%29))
  (bind _returnvalue (Transformation|GetActorLocation))
  (bind (_outhits _returnvalue_2) (Collision|MultiSphereTraceForObjects _returnvalue (+ _returnvalue "0,0,0.100000") 1e+02 (Variables|Default|GetObjectTypes) false 0 "None"))
  (if _returnvalue_2
    (for _array_element _outhits
      (if (== (.hitactor _array_element) (Game|Player|GetPlayerPawn 0))
        (Variables|Default|SetCanObtianKeycard true)
        (if (not (Variables|Default|GetObtained%20Keycard))
          (CallFunction|AddPickupKeycardWidgettoViewport))))
    (else
      (Variables|Default|SetCanObtianKeycard false)
      (CallFunction|RemovePickupKeycardWidgetfromViewport))))

(event Input|ActionEvents|InputActionPickupKeycardAction
  (params (Key :type Key%20Structure :default "None"))
  (bind _returnvalue (Game|GetPlayerCharacter 0))
  (:Pressed
    (if (Variables|Default|GetCanObtianKeycard)
      (Transformation|AttachComponentToComponent (Variables|/Script/Engine.Character|GetMesh _returnvalue) "Key Card Socket" "SnapToTarget" "SnapToTarget" "KeepRelative" true)
      (CallFunction|RemovePickupKeycardWidgetfromViewport)
      (Collision|SetActorEnableCollision false)
      (bind _returnvalue_2 (UserInterface|CreateWidget "/Game/MainLevelUI/YouHavePickedUpTheKeycardWidget.YouHavePickedUpTheKeycardWidget_C"))
      (UserInterface|Viewport|AddtoViewport _returnvalue_2 0)
      (bind _asplayer_base (Utilities|Casting|CastToPlayerBase _returnvalue))
      (Variables|/Script/ActiveShooter.PlayerBase|SetPlayerHasKeycard _asplayer_base true)
      (Variables|Default|SetObtained%20Keycard true))))

(fn ConstructionScript)