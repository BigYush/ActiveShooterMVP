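; BP_RecordingActor is a lobby character actor built from modular skeletal meshes in the MetaHuman style, with no active event logic.
; Its construction script runs the parent's, then makes BodyMesh follow Mesh through master pose.
; Feet, Legs and Torso follow Mesh only if they have a skeletal mesh and neither an anim class nor a post-process AnimBP.
; When Face has a mesh, its eyelash materials become dynamic instances to allow opacity toggling.
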(event EventBeginPlay)

(event Collision|EventActorBeginOverlap
  (params (OtherActor :type Actor%20Object%20Reference)))

(event EventTick
  (params (DeltaSeconds :type Float%20%28single-precision%29)))

(fn ConstructionScript
  (|CallParentFunction)
  (Class|SkinnedMeshComponent|SetMasterPoseComponent (Variables|Default|GetBodyMesh) (Variables|Default|GetMesh) false)
  (CallFunction|EnableMasterPose (Variables|Default|GetFeet))
  (CallFunction|EnableMasterPose (Variables|Default|GetLegs))
  (CallFunction|EnableMasterPose (Variables|Default|GetTorso))
  (Utilities|IsValid (Variables|/Script/Engine.SkinnedMeshComponent|GetSkeletalMesh (Variables|Default|GetFace)) ; Only create MIDs when there is a valid skeletal mesh is set \n(this prevents warnings in MH export)
    (:Is%20Valid
      (Rendering|Material|CreateDynamicMaterialInstance (Variables|Default|GetFace) 6 0 "None" :!class /Script/Engine.PrimitiveComponent) ; Turn eyelashes materials into MIDs so we can toggle opacity when using hair cards
      (Rendering|Material|CreateDynamicMaterialInstance (Variables|Default|GetFace) 10 0 "None" :!class /Script/Engine.PrimitiveComponent))))

(fn EnableMasterPose
  (params (SkeletalMeshComponent :type Skeletal%20Mesh%20Component%20Object%20Reference))
  (bind _skeletalmesh (Variables|/Script/Engine.SkinnedMeshComponent|GetSkeletalMesh SkeletalMeshComponent))
  (if (Utilities|IsValid _skeletalmesh)
    (if (not (or (Utilities|IsValidClass (Variables|/Script/Engine.SkeletalMeshComponent|GetAnimClass SkeletalMeshComponent)) (Utilities|IsValidClass (Variables|/Script/Engine.SkeletalMesh|GetPostProcessAnimBlueprint _skeletalmesh))))
      (Class|SkinnedMeshComponent|SetMasterPoseComponent SkeletalMeshComponent (Variables|Default|GetMesh) false))))