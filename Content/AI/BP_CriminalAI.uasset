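; BP_CriminalAI is the AI controller for criminal NPCs, running BT_CriminalAI on possess and feeding its Blackboard from AI Perception.
; On each perception update it tells senses apart by stimulus array index, with debug prints throughout.
; Index 0 sets or clears CanSeePlayer for any updated actor, without a player check.
; A sensed index 1 (noise) stimulus sets ShouldInvesigate (spelled so) and InvestigateLocation, and never clears them here.
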(event OnPerceptionUpdated(AIPerception)
  (params (UpdatedActors :type Array%20of%20Actor%20Object%20References))
  (bind _returnvalue (AI|GetBlackboard 0))
  (Development|PrintString "OnPerceptionUpdatedCalled")
  (for _array_element UpdatedActors
    (bind _info (Class|AIPerceptionComponent|GetActorsPerception (Variables|Default|GetAIPerception) _array_element))
    (for (_array_element_2 _array_index) (.lastsensedstimuli _info)
      (Utilities|FlowControl|Sequence
        (:then_0
          (if (== _array_index 0)
            (Development|PrintString "0 Executed")
            (if (.bSuccessfullySensed (Utilities|Struct|BreakAIStimulus _array_element_2))
              (Development|PrintString "True AI")
              (AI|Components|Blackboard|SetValueasBool (AI|GetBlackboard 0) (Utilities|Name|MakeLiteralName "CanSeePlayer") true)
              (else
                (Development|PrintString "False AI")
                (AI|Components|Blackboard|SetValueasBool (AI|GetBlackboard 0) (Utilities|Name|MakeLiteralName "CanSeePlayer") false)))))
        (:then_1
          (if (== _array_index 1)
            (Development|PrintString "1 Executed")
            (if (.bSuccessfullySensed (Utilities|Struct|BreakAIStimulus _array_element_2))
              (Development|PrintString "NoiseStimulusDetected")
              (AI|Components|Blackboard|SetValueasBool _returnvalue (Utilities|Name|MakeLiteralName "ShouldInvesigate") true)
              (AI|Components|Blackboard|SetValueasVector _returnvalue (Utilities|Name|MakeLiteralName "InvestigateLocation") (.StimulusLocation (Utilities|Struct|BreakAIStimulus _array_element_2))))))))))

(event EventBeginPlay)

(event EventPossess
  (params (PossessedPawn :type Pawn%20Object%20Reference))
  (AI|RunBehaviorTree "/Game/AI/BT_CriminalAI.BT_CriminalAI"))

(fn ConstructionScript)