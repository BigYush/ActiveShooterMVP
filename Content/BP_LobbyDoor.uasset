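; BP_LobbyDoor is a lobby door that requires the player to hold a keycard.
; Every Tick it runs a debug-drawn multi-sphere trace around itself and checks the hits for the player pawn.
; With PlayerHasKeycard set on PlayerBase, it gives RotatingMovement a yaw rate, which nothing here stops.
; Without the keycard, it adds a new ObtainKeycardToOpenDoor widget on each such hit, with no duplicate guard.
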(event EventBeginPlay)

(event Collision|EventActorBeginOverlap
  (params (OtherActor :type Actor%20Object%20Reference)))

(event EventTick
  (params (DeltaSeconds :type Float%20%28single-precision%29))
  (bind _returnvalue (Transformation|GetActorLocation))
  (bind _returnvalue_2 (Game|Player|GetPlayerPawn 0))
  (bind _outhits (Collision|MultiSphereTraceForObjects _returnvalue (+ _returnvalue "0,0,0.100000") 1.5e+02 (Variables|Default|GetObjectTypes) false 0 "ForOneFrame"))
  (for _array_element _outhits
    (if (== (.hitactor _array_element) _returnvalue_2)
      (bind _asplayer_base (Utilities|Casting|CastToPlayerBase _returnvalue_2))
      (if (Variables|/Script/ActiveShooter.PlayerBase|GetPlayerHasKeycard _asplayer_base)
        (Variables|/Script/Engine.RotatingMovementComponent|SetRotationRate (Variables|Default|GetRotatingMovement) "0,-20.000000, 0")
        (else
          (bind _returnvalue_3 (UserInterface|CreateWidget "/Game/MainLevelUI/ObtainKeycardToOpenDoor.ObtainKeycardToOpenDoor_C"))
          (UserInterface|Viewport|AddtoViewport _returnvalue_3 0))))))

(fn ConstructionScript)